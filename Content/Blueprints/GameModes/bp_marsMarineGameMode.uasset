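; Game mode for the Mars marine game that spawns waves of aliens.
; Shortly after BeginPlay it increments the wave counter once and starts a looping timer for the wave spawn event.
; Each spawn places one BP_Alien at a random TargetPoint, adjusting for collisions.
; A counter check against the current wave follows, but its branch leads nowhere, so no further aliens spawn in that call.
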(event `self.ReceiveBeginPlay`
  (`KismetSystemLibrary.Delay` 2.0)
  (`self.SetupNewWave`))

(event `Spawn Wave`
  (`self.SpawnAliens`))

(fn `GetRandomSpawnLocation`
  (returns (Output :type "TargetPoint Object Reference"))
  (bind _outactors (`GameplayStatics.GetAllActorsOfClass` "/Script/Engine.TargetPoint"))
  (return (`|GetArrayItem` _outactors (`KismetMathLibrary.RandomIntegerInRange` 0 (`KismetArrayLibrary.Array_LastIndex` _outactors)))))

(fn `SetupNewWave`
  (`/Engine/EditorBlueprintResources/StandardMacros.IncrementInt` (`self.CurrentWave`)
    (:`  `
      (`KismetSystemLibrary.K2_SetTimer` null "Spawn Wave" 5.0 true))))

(fn `SpawnAliens`
  (set `self.i` 0)
  (bind _output (`self.GetRandomSpawnLocation`))
  (`/Engine/EditorBlueprintResources/StandardMacros.IsValid` _output
    (:`Is Valid`
      (`|SpawnActorFromClass` "/Game/Blueprints/AI/BP_Alien.BP_Alien_C" (`self.GetTransform` _output) "AdjustIfPossibleButAlwaysSpawn" "OverrideRootScale" null null)
      (bind _newparam (`self.SpawnMoreAliens`))
      (if _newparam
        _))))

(fn `SpawnMoreAliens`
  (returns (NewParam :type Boolean))
  ;[1 1 1] Calculamos si quedan aliens por aparecer en esta ronda.
  (bind _result (`/Engine/EditorBlueprintResources/StandardMacros.IncrementInt` (`self.i`))
    (:`  `
      (return (<= _result (`self.CurrentWave`))))))

(fn `UserConstructionScript`)