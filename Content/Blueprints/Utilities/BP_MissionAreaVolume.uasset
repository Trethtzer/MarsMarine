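; BP_MissionAreaVolume is a volume that marks the playable mission area and punishes the player for leaving it.
; When a bp_marine's overlap ends, it sets that marine's OutsideMissionArea flag and starts a KillPlayer timer lasting TimeBeforePlayerDeath.
; Re-entering clears the flag and cancels the timer.
; On expiry, KillPlayer applies fixed damage to player character 0, regardless of which marine left.
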(event `self.ReceiveActorBeginOverlap`
  (params (OtherActor :type "Actor Object Reference"))
  (bind _asbp_marine (cast `/Game/Blueprints/Pawns/bp_marine` OtherActor))
  (set `/Game/Blueprints/Pawns/bp_marine.OutsideMissionArea` false _asbp_marine)
  (`KismetSystemLibrary.K2_ClearTimer` null "KillPlayer"))

(event `self.ReceiveActorEndOverlap`
  (params (OtherActor :type "Actor Object Reference"))
  (bind _asbp_marine (cast `/Game/Blueprints/Pawns/bp_marine` OtherActor))
  (set `/Game/Blueprints/Pawns/bp_marine.OutsideMissionArea` true _asbp_marine)
  (`KismetSystemLibrary.K2_SetTimer` null "KillPlayer" (`self.timeBeforePlayerDeath`)))

(fn `KillPlayer`
  (`GameplayStatics.ApplyDamage` (`GameplayStatics.GetPlayerCharacter` 0) 100.0))

(fn `UserConstructionScript`)